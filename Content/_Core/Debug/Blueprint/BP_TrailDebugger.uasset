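; BP_TrailDebugger is a debug actor that moves continuously in a horizontal circle, apparently as a moving source for checking trails.
; It caches its spawn location on BeginPlay as the circle's center.
; Each Tick it offsets from that center using cosine and sine of time since creation, scaled by Speed and Radius, and moves there with sweep enabled.
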(event `self.ReceiveBeginPlay`
  (set `self.startPosition` (`self.K2_GetActorLocation`)))

(event `self.ReceiveTick`
  (params (DeltaSeconds :type "Float (single-precision)"))
  (bind _returnvalue (* (`self.GetGameTimeSinceCreation`) (`self.speed`)))
  (`self.K2_SetActorLocation` (+ (* (`KismetMathLibrary.MakeVector` (`KismetMathLibrary.Cos` _returnvalue) (`KismetMathLibrary.Sin` _returnvalue)) (`self.radius`)) (`self.startPosition`)) true))

(fn `UserConstructionScript`)