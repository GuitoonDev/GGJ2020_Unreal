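; GM_NailedIt is the game mode that persists the player's high score and a standing-position flag through a GSave_NailedIt save object.
; On BeginPlay it async-loads the PlayerSavedData slot, or creates and saves a new save object if loading fails.
; It then pushes the high score to the BP_HighScoreDisplayer and tells the MotionControllerPawn to update its starting position.
; SaveGameDatas writes new values and saves them to the slot.
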(event `Save Game Datas`
  (params (`Highest Score` :type Integer) (`Is Stand Position` :type Boolean))
  (bind _savegameinstance (`self.SaveGameInstance`))
  (set `/Game/_core/GPE/SaveScore/GSave_NailedIt.Highest Score` `Highest Score` _savegameinstance)
  (set `/Game/_core/GPE/SaveScore/GSave_NailedIt.IsStandPosition` `Is Stand Position` _savegameinstance)
  (`self.Save Instance`))

(event `self.ReceiveBeginPlay`
  (`self.Load Instance`))

(event `Save Instance`
  (bind _savegameinstance (`self.SaveGameInstance`))
  (`GameplayStatics.SaveGameToSlot` _savegameinstance (`/Game/_core/GPE/SaveScore/GSave_NailedIt.SaveSlotName` _savegameinstance) (`/Game/_core/GPE/SaveScore/GSave_NailedIt.userId` _savegameinstance)))

(event `Load Instance`
  (bind (_savegame _bsuccess) (`AsyncActionHandleSaveGame.AsyncLoadGameFromSlot` "PlayerSavedData")
    (:`Completed`
      (if _bsuccess
        (bind _asgsave_nailed_it (cast `/Game/_core/GPE/SaveScore/GSave_NailedIt` _savegame))
        (set `self.SaveGameInstance` _asgsave_nailed_it)
        (else
          (bind _returnvalue (`GameplayStatics.CreateSaveGameObject` "/Game/_core/GPE/SaveScore/GSave_NailedIt.GSave_NailedIt_C"))
          (bind _output_get (set `self.SaveGameInstance` _returnvalue))
          (`GameplayStatics.SaveGameToSlot` _output_get (`/Game/_core/GPE/SaveScore/GSave_NailedIt.SaveSlotName` _output_get) (`/Game/_core/GPE/SaveScore/GSave_NailedIt.userId` _output_get))))
      (bind _outactors (`GameplayStatics.GetAllActorsOfClass` "/Game/_core/GPE/ScoreDisplayer/BP_HighScoreDisplayer.BP_HighScoreDisplayer_C"))
      (`/Game/_core/GPE/ScoreDisplayer/BP_ScoreDisplayer.SetNewScore` (`|GetArrayItem` _outactors) (`/Game/_core/GPE/SaveScore/GSave_NailedIt.Highest Score` (`self.SaveGameInstance`)))
      (bind _asmotion_controller_pawn (cast `/Game/VirtualRealityBP/Blueprints/MotionControllerPawn` (`GameplayStatics.GetPlayerPawn` 0)))
      (`/Game/VirtualRealityBP/Blueprints/MotionControllerPawn.UpdatePostionAtBegin` _asmotion_controller_pawn))))

(fn `UserConstructionScript`)