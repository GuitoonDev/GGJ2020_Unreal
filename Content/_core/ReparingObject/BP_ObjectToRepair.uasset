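; Repairable object actor that takes on a random mesh and spawns nails on it for a repair task.
; On BeginPlay it picks a random MeshNailsDatabase row for its mesh, material and candidate nail transforms.
; It then spawns a random number of BP_Nail actors from those transforms, removing a separately randomized entry after each, so positions can repeat.
; CheckNailCount decrements the nail counter, but its zero-count branch is empty.
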(event `CheckNailCount`
  (bind _result (`/Engine/EditorBlueprintResources/StandardMacros.DecrementInt` (`self.NailCount`))
    (:`  `
      (if (== _result 0)
        _))))

(event `self.ReceiveBeginPlay`
  (bind _staticmesh (`self.StaticMesh`))
  (bind _returnvalue (`KismetArrayLibrary.Array_Length` (`self.NailSpawnTransformArray`)))
  (bind _returnvalue_2 (`KismetMathLibrary.RandomInteger` _returnvalue))
  (bind (_output_location _output_rotation _output_scale) (`KismetMathLibrary.BreakTransform` (`|GetArrayItem` (`self.NailSpawnTransformArray`) _returnvalue_2)))
  (`|ExecutionSequence`
    (:`then_0`
      (bind _outrownames (`DataTableFunctionLibrary.GetDataTableRowNames` "/Game/_core/ReparingObject/StructAndDatabase/MeshNailsDatabase.MeshNailsDatabase"))
      (bind _returnvalue_3 (`|GetDataTableRow` "/Game/_core/ReparingObject/StructAndDatabase/MeshNailsDatabase.MeshNailsDatabase" (`|GetArrayItem` _outrownames (`KismetMathLibrary.RandomInteger` (`KismetArrayLibrary.Array_Length` _outrownames))))
        (:`then`
          (`StaticMeshComponent.SetStaticMesh` _staticmesh (break `/Game/_core/ReparingObject/StructAndDatabase/MeshNailPositionStruct` _returnvalue_3))
          (`PrimitiveComponent.SetMaterial` _staticmesh 0 (`.Material_10_D56671894A630BF83430D29599032D8D` (break `/Game/_core/ReparingObject/StructAndDatabase/MeshNailPositionStruct` _returnvalue_3)))
          (set `self.NailSpawnTransformArray` (`.Positions_6_2B062FF74275AA4D0F15998D45EE039B` (break `/Game/_core/ReparingObject/StructAndDatabase/MeshNailPositionStruct` _returnvalue_3))))))
    (:`then_1`
      (bind _output_get (set `self.NailCount` (`KismetMathLibrary.RandomIntegerInRange` 2 _returnvalue)))
      (for _ (range _output_get)
        (`|SpawnActorFromClass` "/Game/_core/Nail/BP_Nail.BP_Nail_C" (`KismetMathLibrary.MakeTransform` (+ _output_location (`SceneComponent.K2_GetComponentLocation` (`self.StaticMesh`))) _output_rotation _output_scale) "AlwaysSpawn" "OverrideRootScale" null null)
        (`KismetArrayLibrary.Array_Remove` (`self.NailSpawnTransformArray`) _returnvalue_2)))))

(fn `UserConstructionScript`)