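; BP_ObjectToRepair is a repairable object that tracks its remaining nails and sets IsCompleted when CheckNailCount counts them down to zero.
; An unconnected setup chain picks a random mesh, materials and nail transforms from the MeshNailsDatabase table, then spawns a random number of BP_Nail actors.
; That chain never runs, as BeginPlay is empty, and its separate random index picks can mismatch spawned and removed transforms.
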(event `CheckNailCount`
  (bind _result (`/Engine/EditorBlueprintResources/StandardMacros.DecrementInt` (`self.NailCount`))
    (:`  `
      (if (== _result 0)
        ;[1 1 1] Add Feedbacks here
        (set `self.IsCompleted` true)))))

(event `self.ReceiveBeginPlay`)

(fn `UserConstructionScript`)