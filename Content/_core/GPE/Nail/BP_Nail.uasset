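; BP_Nail is a nail that a motion controller smashes as part of repairing an object.
; The first box overlap by a BP_MotionController fires OnNailSmashed once.
; That event calls CheckNailCount on the referenced object to repair, spawns a Niagara hammer-impact effect and sinks the nail pivot along its up vector.
; HasValidDirection tests strike direction and speed, but its call is unwired, so any such overlap counts.
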(event `OnNailSmashed`
  (bind _nail_pivot (`self.Nail Pivot`))
  (`/Game/_core/GPE/ReparingObject/BP_ObjectToRepair.CheckNailCount` (`self.ObjectToRepairReference`))
  ;[1 1 1] Add Feedbacks here --> Enfoncer le clou, jouer le son et instantier les fxs
  (`NiagaraFunctionLibrary.SpawnSystemAtLocation` "/Game/_core/VFX/Hammer/HammerImpact/NS_HammerImpact.NS_HammerImpact" (`self.K2_GetActorLocation`) (`self.K2_GetActorRotation`))
  (`SceneComponent.K2_SetWorldLocation` (`self.Nail Pivot`) (- (`SceneComponent.K2_GetComponentLocation` _nail_pivot) (* (`SceneComponent.GetUpVector` _nail_pivot) 15.0)) false false))

(event `self.BoxCollision.OnComponentBeginOverlap`
  (params (OverlappedComponent :type "PrimitiveComponent Object Reference") (OtherActor :type "Actor Object Reference") (OtherComp :type "PrimitiveComponent Object Reference") (OtherBodyIndex :type Integer) (bFromSweep :type Boolean) (SweepResult :type "HitResult Structure (by ref)"))
  (bind _asbp_motion_controller (cast `/Game/VirtualRealityBP/Blueprints/BP_MotionController` OtherActor))
  (`/Engine/EditorBlueprintResources/StandardMacros.DoOnce` false
    (:`Completed`
      (`self.OnNailSmashed`))))

(fn `HasValidDirection `
  (params (LimitAngle :type "Float (double-precision)") (LimitVelocity :type "Float (double-precision)") (InDirection :type "Vector Structure"))
  (returns (IsValid :type Boolean))
  (bind _returnvalue (* (`KismetMathLibrary.Dot_VectorVector` InDirection (`self.GetActorUpVector`)) 90.0))
  (`KismetSystemLibrary.PrintString` (`KismetStringLibrary.Conv_DoubleToString` _returnvalue) true true (struct :`R` 1.0 :`G` 0.688079 :`A` 1.0) 1.0)
  (return (and (> LimitAngle _returnvalue) (> (`KismetMathLibrary.VSize` InDirection) LimitVelocity))))

(fn `UserConstructionScript`)