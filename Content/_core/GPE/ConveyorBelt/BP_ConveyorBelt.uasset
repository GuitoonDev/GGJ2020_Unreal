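; Conveyor belt for the NailedIt game that brings in objects to repair, adding score when the current one is completed and removing a life otherwise.
; Each check spawns a new object with a sound, then timelines lerp meshes between spawn and despawn points, the current one half a belt ahead.
; A material parameter collection pans the belt texture alongside.
; Destroying and replacing the outgoing object is left unwired.
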(event `CheckCurrentObject`
  (bind _currentobject_ (`self.CurrentObject `))
  (`/Engine/EditorBlueprintResources/StandardMacros.IsValid` _currentobject_
    (:`Is Valid`
      (bind _asgs_nailed_it (cast `/Game/_Core/GameState/GS_NailedIt` (`GameplayStatics.GetGameState`)))
      (if (`/Game/_Core/GPE/ReparingObject/BP_ObjectToRepair.IsCompleted` _currentobject_)
        ;[1 1 1] Increase Score
        (`/Game/_Core/GameState/GS_NailedIt.IncreaseScore` _asgs_nailed_it 0)
        (`self.SpawnNextObject`)
        (else
          ;[1 1 1] Decrease Life
          (`/Game/_Core/GameState/GS_NailedIt.RemoveLifePoint` _asgs_nailed_it)
          (`self.SpawnNextObject`))))
    (:`Is Not Valid`
      (`self.SpawnNextObject`))))

(event `SpawnNextObject`
  (bind _returnvalue_location (`KismetMathLibrary.BreakTransform` (`SceneComponent.K2_GetComponentToWorld` (`self.SpawnPosition`))))
  (`GameplayStatics.SpawnSoundAtLocation` "/Game/_Core/Audio/Tapis/ConveyorBeltCue.ConveyorBeltCue" (0.0 0.0 0.0) (struct) 1.0 1.0 0.0 null null)
  (bind _returnvalue (`|SpawnActorFromClass` "/Game/_Core/GPE/ReparingObject/BP_ObjectToRepair.BP_ObjectToRepair_C" (`KismetMathLibrary.MakeTransform` _returnvalue_location (struct :`Yaw` 90.0)) "Undefined" "OverrideRootScale" null null))
  (set `self.NextObject` _returnvalue)
  (`/Engine/EditorBlueprintResources/StandardMacros.IsValid` (`self.CurrentObject `)
    (:`Is Valid`
      (bind (_direction _movementtimeline) (`Timeline|MovementTimeLine` :!via `PlayFromStart`)
        (:`Update`
          (`self.MoveNextObject` _movementtimeline)
          (`self.MoveCurrentObject` _movementtimeline)
          (`KismetMaterialLibrary.SetScalarParameterValue` "/Game/_Core/GPE/ConveyorBelt/MPC_ConveyorMaterialParameters.MPC_ConveyorMaterialParameters" "Pan" (+ (* _movementtimeline (`self.panAmount`)) (`self.texturePanOffset`))))
        (:`Finished`
          (set `self.texturePanOffset` (/ (`self.panAmount`) 2.0)) ; Offsets the pan with the previous reached distance
          (`KismetSystemLibrary.PrintString` "Hello"))))
    (:`Is Not Valid`
      (bind (_direction_2 _movementtimeline_2) (`Timeline|MovementTimeLineBis` :!via `PlayFromStart`)
        (:`Update`
          (`self.MoveNextObject` _movementtimeline_2)
          (set `self.CurrentObject ` (`self.NextObject`)))))))

(event `MoveNextObject`
  (params (Delta :type "Float (double-precision)"))
  ;[0 0 0] Apply Movements
  (`SceneComponent.K2_SetWorldLocation` (`/Game/_Core/GPE/ReparingObject/BP_ObjectToRepair.StaticMesh` (`self.NextObject`)) (`KismetMathLibrary.VLerp` (`SceneComponent.K2_GetComponentLocation` (`self.SpawnPosition`)) (`SceneComponent.K2_GetComponentLocation` (`self.DeSpawnPosition`)) Delta) false false))

(event `MoveCurrentObject`
  (params (Delta :type "Float (double-precision)"))
  ;[0 0 0] Apply Movements
  (`SceneComponent.K2_SetWorldLocation` (`/Game/_Core/GPE/ReparingObject/BP_ObjectToRepair.StaticMesh` (`self.CurrentObject `)) (`KismetMathLibrary.VLerp` (`SceneComponent.K2_GetComponentLocation` (`self.SpawnPosition`)) (`SceneComponent.K2_GetComponentLocation` (`self.DeSpawnPosition`)) (+ Delta 0.5)) false false))

(fn `UserConstructionScript`)