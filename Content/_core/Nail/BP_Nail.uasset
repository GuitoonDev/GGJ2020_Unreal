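; BP_Nail is a nail that the player smashes with a motion controller as part of repairing an object.
; A hit on its box collision by a BP_MotionController triggers OnNailSmashed through a DoOnce, so it fires a single time.
; That event calls CheckNailCount on the referenced object to repair and sinks the mesh one unit along its down axis.
; Sound and FX feedback are only a placeholder comment.
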(event `OnNailSmashed`
  (bind _staticmesh (`self.StaticMesh`))
  (`/Game/_core/ReparingObject/BP_ObjectToRepair.CheckNailCount` (`self.ObjectToRepairReference`))
  ;[1 1 1] Add Feedbacks here --> Enfoncer le clou, jouer le son et instantier les fxs
  (`SceneComponent.K2_SetWorldLocation` _staticmesh (- (`SceneComponent.K2_GetComponentLocation` _staticmesh) (`SceneComponent.GetUpVector` _staticmesh)) false false))

(event `self.BoxCollision.OnComponentHit`
  (params (HitComponent :type "PrimitiveComponent Object Reference") (OtherActor :type "Actor Object Reference") (OtherComp :type "PrimitiveComponent Object Reference") (NormalImpulse :type "Vector Structure") (Hit :type "HitResult Structure (by ref)"))
  (cast `/Game/VirtualRealityBP/Blueprints/BP_MotionController` OtherActor)
  (`/Engine/EditorBlueprintResources/StandardMacros.DoOnce` false
    (:`Completed`
      (`self.OnNailSmashed`))))

(fn `UserConstructionScript`)